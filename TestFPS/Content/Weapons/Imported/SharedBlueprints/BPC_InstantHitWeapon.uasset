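; Base Blueprint actor for an instant-hit weapon that defines the firing sequence as a template.
; OnFire checks CanWeaponFire, then decrements ammo, plays muzzle flash and sound, determines hit objects and applies damage if any are found.
; Each step is a separate stub function: both checks return false, so firing does nothing as written.
; PlayNoAmmoSound is present but not connected to the firing flow.
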(event Custom|OnFire
  (bind _canfire (CallFunction|CanWeaponFire))
  (if _canfire
    (CallFunction|DecrementAmmo)
    (CallFunction|PlayMuzzleFlash)
    (CallFunction|PlayFireSound)
    (bind _hitoccurred (CallFunction|DetermineHitObjects))
    (if _hitoccurred
      (CallFunction|ApplyDamagetoHitActors))))

(event EventBeginPlay)

(event Collision|EventActorBeginOverlap
  (params (OtherActor :type Actor%20Object%20Reference)))

(event EventTick
  (params (DeltaSeconds :type Float%20%28single-precision%29))
  (|CallParentFunction 0.0))

(fn ConstructionScript
  (|CallParentFunction))

(fn CanWeaponFire
  (return false))

(fn DecrementAmmo)

(fn PlayNoAmmoSound)

(fn PlayMuzzleFlash)

(fn PlayFireSound)

(fn DetermineHitObjects
  (return false))

(fn ApplyDamagetoHitActors)